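; Speed power-up pickup that gives a temporary boost to whichever of the two player physics balls touches it.
; On mesh overlap it casts to PhysicsBallBP1, falling back to PhysicsBallBP2, and turns that ball's speed power function on.
; It then destroys its mesh and light so it vanishes, while the actor stays alive to switch the boost off after a five-second delay.
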(event `self.ReceiveTick`
  (params (DeltaSeconds :type "Float (single-precision)")))

(event `self.StaticMesh.OnComponentBeginOverlap`
  (params (OverlappedComponent :type "PrimitiveComponent Object Reference") (OtherActor :type "Actor Object Reference") (OtherComp :type "PrimitiveComponent Object Reference") (OtherBodyIndex :type Integer) (bFromSweep :type Boolean) (SweepResult :type "HitResult Structure (by ref)"))
  (bind _asphysics_ball_bp1 (cast `/Game/RollingBP/Blueprints/PhysicsBallBP1` OtherActor)
    (:`then`
      (`/Game/RollingBP/Blueprints/PhysicsBallBP1.SpeedPowerFunc` _asphysics_ball_bp1 true)
      (`ActorComponent.K2_DestroyComponent` (`self.StaticMesh`))
      (`ActorComponent.K2_DestroyComponent` (`self.PointLight`))
      (`KismetSystemLibrary.Delay` 5.0)
      (`/Game/RollingBP/Blueprints/PhysicsBallBP1.SpeedPowerFunc` _asphysics_ball_bp1 false))
    (:`CastFailed`
      (bind _asphysics_ball_bp2 (cast `/Game/RollingBP/Blueprints/PhysicsBallBP2` OtherActor))
      (`/Game/RollingBP/Blueprints/PhysicsBallBP2.SpeedPowerFuncP2` _asphysics_ball_bp2 true)
      (`ActorComponent.K2_DestroyComponent` (`self.StaticMesh`))
      (`ActorComponent.K2_DestroyComponent` (`self.PointLight`))
      (`KismetSystemLibrary.Delay` 5.0)
      (`/Game/RollingBP/Blueprints/PhysicsBallBP2.SpeedPowerFuncP2` _asphysics_ball_bp2 false))))

(fn `UserConstructionScript`)